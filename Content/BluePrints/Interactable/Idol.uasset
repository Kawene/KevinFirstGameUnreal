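; Interactable idol that starts an enemy-style wave encounter and, once it can be picked up, unlocks the end of the game.
; Interacting while locked starts a looping SpawnWave timer, with a negative start delay offsetting the first interval.
; SpawnWave triggers WaveSpawners for a single wave, then on the next tick pauses the timer and makes the idol pickable.
; Interacting then destroys it and sets CanEndTheGame on the EndGame actor.
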(event Custom|SpawnWave
  (if (< (Variables|Default|GetWaveCount) 1)
    (Default|Spawns (Variables|Default|GetWaveSpawners))
    (bind _result (Math|Integer|IncrementInt (stale _output_get))
      (:%20%20
        (bind _output_get (Variables|Default|SetWaveCount _result))))
    (else
      (Class|KismetSystemLibrary|PauseTimer 0 "SpawnWave")
      (Variables|Default|SetCanBePicked true))))

(event EventInteract
  (if (Variables|Default|GetCanBePicked)
    (Actor|DestroyActor)
    (bind _returnvalue (Actor|GetActorOfClass "/Game/BluePrints/MapInteraction/EndGame.EndGame_C"))
    (Variables|/Game/BluePrints/MapInteraction/EndGame.EndGame_C|SetCanEndTheGame _returnvalue true)
    (else
      (Utilities|Time|SetTimerbyFunctionName 0 "SpawnWave" 15.0 true false -15.0))))

(fn ConstructionScript)