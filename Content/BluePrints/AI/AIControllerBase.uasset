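; AIControllerBase is an AI controller that runs the BasicBehavior tree and shares player detection with all AI controllers of its class.
; When perception updates on a Player while its Blackboard TargetPlayer is unset, it calls PlayerFound on every AIControllerBase in the world, setting each one's TargetPlayer.
; Its Death event detaches the controlled pawn pending destruction, then destroys the controller.
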(event OnTargetPerceptionUpdated(AIPerception)
  (params (Actor :type Actor%20Object%20Reference) (Stimulus :type AI%20Stimulus%20Structure))
  (Utilities|IsValid (AI|Components|Blackboard|GetValueasObject (Variables|Default|GetBlackboard) (Utilities|Name|MakeLiteralName "TargetPlayer"))
    (:Is%20Not%20Valid
      (bind _asplayer (Utilities|Casting|CastToPlayer Actor))
      (bind _outactors (Actor|GetAllActorsOfClass "AIControllerBase_C"))
      (for _array_element _outactors
        (CallFunction|PlayerFound _array_element _asplayer)))))

(event Custom|Death
  (Class|Pawn|DetachfromControllerPendingDestroy (Pawn|GetControlledPawn))
  (Actor|DestroyActor))

(event EventBeginPlay
  (AI|RunBehaviorTree "/Game/BluePrints/AI/BasicBehavior.BasicBehavior"))

(fn ConstructionScript)

(fn PlayerFound
  (params (Player :type Player%20Object%20Reference))
  (AI|Components|Blackboard|SetValueasObject (Variables|Default|GetBlackboard) (Utilities|Name|MakeLiteralName "TargetPlayer") Player))