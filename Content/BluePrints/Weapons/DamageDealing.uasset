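; DamageDealing is a melee weapon actor that applies a position offset and attaches to its owner's right-hand socket on Init.
; While attacking, Tick box-traces between two hitbox components on the Camera channel, ignoring the owner.
; Actors with a HealthComponent on another team take damage, with a flesh-hit sound at the end hitbox.
; An ActorHits list, cleared by each Attack event, limits each target to one hit per attack.
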(event Custom|Attack
  (Utilities|Array|Clear (Variables|Default|GetActorHits)))

(event EventTick
  (params (DeltaSeconds :type Float%20%28single-precision%29))
  (if (Variables|Default|GetIsAttacking)
    (bind (_outhits _returnvalue) (Class|KismetSystemLibrary|BoxTraceMulti (Transformation|GetWorldLocation (Variables|Default|GetStartHitBox)) (Transformation|GetWorldLocation (Variables|Default|GetEndHitBox)) "10.000000,10.000000,10.000000" "0, 0, 0" "TraceTypeQuery2" false (Utilities|Array|MakeArray (Variables|Default|GetWeaponOwner)) "None" true))
    (if _returnvalue
      (for _array_element _outhits
        (Utilities|IsValid (Actor|GetComponentbyClass (.HitActor (Collision|BreakHitResult _array_element)) "/Game/BluePrints/BluePrintComponent/HealthComponent.HealthComponent_C")
          (:Is%20Valid
            (if (!= (Variables|Default|GetTeam) (Variables|/Game/BluePrints/BluePrintComponent/HealthComponent.HealthComponent_C|GetTeam (Actor|GetComponentbyClass (.HitActor (Collision|BreakHitResult _array_element)) "/Game/BluePrints/BluePrintComponent/HealthComponent.HealthComponent_C")))
              (if (not (Utilities|Array|ContainsItem (Variables|Default|GetActorHits) (.HitActor (Collision|BreakHitResult _array_element))))
                (Default|ApplyHealthChanges (Actor|GetComponentbyClass (.HitActor (Collision|BreakHitResult _array_element)) "/Game/BluePrints/BluePrintComponent/HealthComponent.HealthComponent_C") (Variables|Default|GetDamageValue) "0, 0, 0")
                (Utilities|Array|Add (Variables|Default|GetActorHits) (.HitActor (Collision|BreakHitResult _array_element)))
                (Audio|PlaySoundatLocation "/Game/Sound/Effects/Weapons/HittingFlesh.HittingFlesh" (Transformation|GetWorldLocation (Variables|Default|GetEndHitBox)) "0, 0, 0" 1.0 1.0 0.0 0 0 0 0)))))))))

(fn ConstructionScript)

(fn Init
  (params (Owner :type Base%20Character%20Object%20Reference))
  (Utilities|FlowControl|Sequence
    (:then_0
      (Transformation|SetActorLocation (Variables|Default|GetPositionOffset) false false))
    (:then_1
      (Variables|Default|SetWeaponOwner Owner))
    (:then_2
      (Transformation|AttachComponentToComponent (Variables|/Script/Engine.Character|GetMesh Owner) "hand_r" "KeepRelative" "SnapToTarget" "SnapToTarget" true))))