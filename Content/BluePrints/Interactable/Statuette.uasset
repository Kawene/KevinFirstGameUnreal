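; Interactable statuette that serves as a dungeon objective, starting enemy-style spawn waves and later becoming the pickup that unlocks the ending.
; The first interaction makes it glow, plays a choir sound and starts a looping timer that triggers WaveSpawners, offset to fire immediately.
; After the final wave spawns, the timer pauses, the material changes and pickup is enabled.
; Taking it destroys the actor, enables EndGame and updates the player's objective to exit.
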(event Custom|SpawnWave
  (Default|Spawns (Variables|Default|GetWaveSpawners))
  (bind _result (Math|Integer|IncrementInt (stale _output_get))
    (:%20%20
      (bind _output_get (Variables|Default|SetWaveCount _result))
      (if (>= _output_get 4)
        (CallFunction|EndWaveSpawning)
        (bind _asplayer (Utilities|Casting|CastToPlayer (Game|GetPlayerCharacter 0)))
        (Default|SetObjectiveText _asplayer (Variables|Default|GetObjectiveText))))))

(event EventInteract
  (if (Variables|Default|GetCanBePicked)
    (CallFunction|IdolTaken)
    (else
      (CallFunction|FirstInteraction)))
  (bind _asplayer (Utilities|Casting|CastToPlayer (Game|GetPlayerCharacter 0)))
  (Default|SetObjectiveText _asplayer (Variables|Default|GetObjectiveText)))

(fn ConstructionScript)

(fn IdolTaken
  (Actor|DestroyActor)
  (bind _returnvalue (Actor|GetActorOfClass "/Game/BluePrints/MapInteraction/EndGame.EndGame_C"))
  (Variables|/Game/BluePrints/MapInteraction/EndGame.EndGame_C|SetCanEndTheGame _returnvalue true)
  (Variables|Default|SetObjectiveText "Exit the dungeon!!"))

(fn FirstInteraction
  (Utilities|FlowControl|DoOnce false
    (:Completed
      (Utilities|Time|SetTimerbyFunctionName 0 "SpawnWave" 15.0 true false -15.0)
      (Rendering|Material|SetMaterial (Variables|Default|GetStaticMesh) 0 "/Game/Material/GlowingIdol.GlowingIdol")
      (Audio|PlaySoundatLocation "/Game/Sound/Effects/Idol/short-choir-6116_Cue.short-choir-6116_Cue" (Transformation|GetActorLocation) "0, 0, 0" 1.0 1.0 0.0 0 0 0 0))))

(fn EndWaveSpawning
  (Class|KismetSystemLibrary|PauseTimer 0 "SpawnWave")
  (Variables|Default|SetCanBePicked true)
  (Variables|Default|SetObjectiveText "Take the statuette")
  (Rendering|Material|SetMaterial (Variables|Default|GetStaticMesh) 0 "/Game/Material/Material_Maps/Level1/M_Statue_Hooded_Metal_Inst.M_Statue_Hooded_Metal_Inst"))