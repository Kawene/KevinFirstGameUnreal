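; Actor component that tracks health for BaseCharacter owners and handles damage and death.
; ApplyHealthChanges subtracts damage from CurrentHealth, capped only at MaxHealth, so negative damage can heal up to that limit.
; It then casts the owner to BaseCharacter, calls DamageRecieved on every change, and calls Death with the hit direction once health reaches zero or below.
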(event EventBeginPlay)

(event EventTick
  (params (DeltaSeconds :type Float%20%28single-precision%29)))

(fn ApplyHealthChanges
  (params (Damage :type Float%20%28double-precision%29) (Direction :type Vector))
  (Variables|Default|Set_currentHealth (Math|Float|Min(Float) (- (Variables|Default|Get_currentHealth) Damage) (Variables|Default|Get_maxHealth)))
  (bind _asbase_character (Utilities|Casting|CastToBaseCharacter (Components|GetOwner)))
  (Default|DamageRecieved _asbase_character)
  (if (<= (Variables|Default|Get_currentHealth) 0.0)
    (Default|Death _asbase_character Direction)))