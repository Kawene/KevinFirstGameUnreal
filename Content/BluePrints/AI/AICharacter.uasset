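; AI enemy character Blueprint that fights with a sword and periodically makes monster noises.
; BeginPlay spawns the sword on the HealthComponent's team and caches the EnemyAnimations instance, which LightAttack triggers alongside an attack sound and the weapon attack.
; A Delay inside Tick spaces the ambient noises at random intervals.
; Death disables tick, silencing further noises, and notifies the AIControllerBase before calling the parent death logic.
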(event EventBeginPlay
  (CallFunction|SpawnWeapon "/Game/BluePrints/Weapons/EnemySword.EnemySword_C" (Variables|/Game/BluePrints/BluePrintComponent/HealthComponent.HealthComponent_C|GetTeam (Variables|Default|GetHealthComponent)))
  (bind _asenemy_animations (Utilities|Casting|CastToEnemyAnimations (Components|SkeletalMesh|GetAnimInstance (Variables|Character|GetMesh))))
  (Variables|Default|SetAnim%20Ref _asenemy_animations))

(event EventTick
  (params (DeltaSeconds :type Float%20%28single-precision%29))
  (Utilities|FlowControl|Delay (Math|Random|RandomFloatinRange 1e+01 2e+01))
  (if (Class|Actor|IsActorTickEnabled)
    (Audio|PlaySoundatLocation "/Game/Sound/Effects/MonsterRoarsAndGrowls/RandomMonsterNoise.RandomMonsterNoise" (Transformation|GetActorLocation) "0, 0, 0" 1.0 1.0 0.0 0 0 0 0)))

(fn ConstructionScript
  (|CallParentFunction))

(fn LightAttack
  (Audio|PlaySoundatLocation "/Game/Sound/Effects/MonsterRoarsAndGrowls/AttackMonster.AttackMonster" (Transformation|GetActorLocation) "0, 0, 0" 1.0 1.0 0.0 0 0 0 0)
  (Default|LightAttack (Variables|Default|GetAnim%20Ref))
  (Default|Attack (Variables|Default|GetWeapon)))

(fn Death
  (params (Direction :type Vector :default "0, 0, 0"))
  (Actor|Tick|SetActorTickEnabled false)
  (bind _asaicontroller_base (Utilities|Casting|CastToAIControllerBase (Pawn|GetController)))
  (Default|Death _asaicontroller_base)
  (|CallParentFunction Direction))