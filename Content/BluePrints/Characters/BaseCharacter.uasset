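; Base character Blueprint for melee combat, providing weapon spawning, a light attack, hit feedback and death handling.
; On BeginPlay it spawns a Sword assigned to a team, stores it as Weapon and initializes it with itself as owner.
; LightAttack plays the ChainAttack montage and triggers the weapon's attack.
; DamageRecieved activates a blood effect, while Death destroys the capsule and ragdolls the mesh through physics simulation.
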(event EventBeginPlay
  (CallFunction|SpawnWeapon "/Game/BluePrints/Weapons/Sword.Sword_C"))

(fn ConstructionScript)

(fn SpawnWeapon
  (params (WeaponType :type Damage%20Dealing%20Class%20Reference) (Team :type Integer))
  (bind _returnvalue (Game|SpawnActorfromClass WeaponType (Transformation|GetActorTransform) "Undefined" "MultiplyWithRoot" 0 Team 0))
  (bind _output_get (Variables|Default|SetWeapon _returnvalue))
  (Default|Init _output_get self))

(fn LightAttack
  (Animation|Montage|MontagePlay (Components|SkeletalMesh|GetAnimInstance (Variables|Character|GetMesh)) "/Game/Animations/Knight/ChainAttack.ChainAttack" 1.0 "MontageLength" 0.0 true)
  (Default|Attack (Variables|Default|GetWeapon)))

(fn Death
  (Components|DestroyComponent (Variables|Collision|GetCapsuleComponent))
  (Physics|SetSimulatePhysics (Variables|Character|GetMesh) true))

(fn DamageRecieved
  (Components|Activation|Activate (Variables|Default|GetBloodEffect) true))