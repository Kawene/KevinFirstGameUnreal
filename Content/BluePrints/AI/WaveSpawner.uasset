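; WaveSpawner is a trigger actor that fires a group of AI spawners as a wave.
; The first player overlap, gated by a one-shot ShouldSpawed flag, spawns AI without knowledge of the player's location.
; The Spawns event skips that gate, looks up the Player actor and spawns AI that know its location.
; Both paths use UseSpawners, which calls SpawnAi on every entry in Spawners.
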(event Custom|Spawns
  (bind _returnvalue (Actor|GetActorOfClass "/Game/BluePrints/Characters/Player/Player.Player_C"))
  (CallFunction|UseSpawners true _returnvalue))

(event Collision|EventActorBeginOverlap
  (params (OtherActor :type Actor%20Object%20Reference))
  (bind _asplayer (Utilities|Casting|CastToPlayer OtherActor))
  (if (Variables|Default|GetShouldSpawed)
    (Variables|Default|SetShouldSpawed false)
    (CallFunction|UseSpawners false _asplayer)))

(fn ConstructionScript)

(fn UseSpawners
  (params (KnowPlayersLocation :type Boolean) (Player :type Player%20Object%20Reference))
  (for _array_element (Variables|Default|GetSpawners)
    (Default|SpawnAi _array_element KnowPlayersLocation Player)))